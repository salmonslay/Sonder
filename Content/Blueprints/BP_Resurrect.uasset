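; Resurrection point actor that revives a dead Soul or Robot character when a PROJCharacter overlaps it.
; Its Sphere hides 3.5 seconds after BeginPlay, reappears on the Playerdied event, and hides again after a revive.
; On overlap, it checks the first BP_SoulCharacter and BP_ThirdPersonCharacter found, calling Resurrect on whichever is dead.
; Older scale-based death checks and BP_ArenaFailHandler notifications remain as disconnected nodes.
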(event Custom|Player%20died
  (Development|SetHiddeninGame (Variables|Default|GetSphere) false false))

(event EventBeginPlay
  (Utilities|FlowControl|Delay 3.5)
  (Development|SetHiddeninGame (Variables|Default|GetSphere) true false))

(event Collision|EventActorBeginOverlap
  (params (OtherActor :type Actor%20Object%20Reference))
  (Utilities|Casting|CastToPROJCharacter OtherActor)
  (if true
    ;[1 1 1] Resurrect function
    (Utilities|FlowControl|Sequence
      (:then_0
        (bind _outactors (Actor|GetAllActorsOfClass "/Game/Blueprints/BP_SoulCharacter.BP_SoulCharacter_C"))
        (if (|CheckifSouldead (Utilities|Array|Get(acopy) _outactors))
          (Default|Resurrect (Utilities|Array|Get(acopy) _outactors))
          (Development|SetHiddeninGame (Variables|Default|GetSphere) true false :!label _label)))
      (:then_1
        (bind _outactors_2 (Actor|GetAllActorsOfClass "/Game/ThirdPerson/Blueprints/BP_ThirdPersonCharacter.BP_ThirdPersonCharacter_C"))
        (if (|CheckifRobotdead (Utilities|Array|Get(acopy) _outactors_2))
          (Default|Resurrect (Utilities|Array|Get(acopy) _outactors_2))
          (goto _label))))))

(event EventTick
  (params (DeltaSeconds :type Float%20%28single-precision%29)))

(fn ConstructionScript)