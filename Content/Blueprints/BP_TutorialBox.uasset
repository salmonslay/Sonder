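; BP_TutorialBox is a trigger actor that shows a tutorial popup the first time the player enters it.
; On overlap with an actor tagged Player, a HasShowedTutorial flag ensures the popup fires only once.
; It finds top-level UWBP_Game widgets at runtime, prints their count for debugging, and calls OpenTutorialPopup on each with its TutorialImage.
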(event Collision|EventActorBeginOverlap
  (params (OtherActor :type Actor%20Object%20Reference))
  (if (Actor|ActorHasTag OtherActor "Player")
    (if (not (Variables|Default|GetHas%20showed%20tutorial?))
      (Variables|Default|SetHas%20showed%20tutorial? true)
      (bind _foundwidgets (Widget|GetAllWidgetsOfClass "/Game/UI/Gameplay/UWBP_Game.UWBP_Game_C" true))
      (Development|PrintString (Utilities|String|Append "Widget count: " (Utilities|String|ToString(Integer) (Utilities|Array|Length _foundwidgets))))
      (for _array_element _foundwidgets
        (Default|OpenTutorialPopup🏫🎒 _array_element (Variables|Default|GetTutorial%20image))))))

(fn ConstructionScript)