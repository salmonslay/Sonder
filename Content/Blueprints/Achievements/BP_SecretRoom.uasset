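; BP_SecretRoom is a secret-room trigger that grants an achievement and unlocks the football.
; It tracks overlapping PROJCharacters in an Overlappers list, removing actors when they leave.
; The reward fires when AddUnique returns index 1, meaning a second character joins one already inside.
; It then caches and writes the secret-room achievement for player controller 0, and sets FootballUnlocked in the save game.
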(event Collision|EventActorBeginOverlap
  (params (OtherActor :type Actor%20Object%20Reference))
  (Utilities|Casting|CastToPROJCharacter OtherActor)
  (bind _returnvalue (Utilities|Array|AddUnique (Variables|Default|GetOverlappers) OtherActor))
  (if (== _returnvalue 1)
    (Utilities|FlowControl|Sequence
      (:then_0
        (|CacheAchievements (Game|GetPlayerController 0)
          (:OnSuccess
            (|WriteAchievementProgress (Game|GetPlayerController 0) "ACHIEVEMENT_SECRETROOM" 1.0))))
      (:then_1
        (bind _output_get (Variables|Default|SetSave (Class|PROJCharacter|GetSaveGameSafe)))
        (Variables|/Script/Sonder.SonderSaveGame|SetbFootballUnlocked _output_get true)
        (Class|PROJCharacter|SetSaveGame _output_get)))))

(event Collision|EventActorEndOverlap
  (params (OtherActor :type Actor%20Object%20Reference))
  (Utilities|Array|RemoveItem (Variables|Default|GetOverlappers) OtherActor))

(fn ConstructionScript)