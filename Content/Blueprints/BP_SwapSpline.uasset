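; BP_SwapSpline is a platform trigger that fires a spline swap once the required number of player characters stand on it.
; BeginPlay sets that requirement to one or two from NeedTwoPlayers.
; Overlapping PROJCharacters are added to an array, and an exact count match calls SplineSwap, with debug prints either way.
; Leaving removes the last array entry regardless of who left; both RepNotify functions are empty.
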(event Custom|CheckSwap
  (if (== (Utilities|Array|Length (Variables|Default|GetThings%20On%20Platform)) (Variables|Default|GetAmount%20Needed%20on%20Platform))
    (Class|SwapSpline|SplineSwap)
    (Development|PrintString "Hello")
    (else
      (Development|PrintString "No"))))

(event EventBeginPlay
  (if (Variables|Default|GetNeed%20Two%20Players)
    (Variables|Default|SetAmount%20Needed%20on%20Platform 2)
    (else
      (Variables|Default|SetAmount%20Needed%20on%20Platform 1))))

(event Collision|EventActorEndOverlap
  (params (OtherActor :type Actor%20Object%20Reference))
  (bind _things_on_platform (Variables|Default|GetThings%20On%20Platform))
  (Utilities|Casting|CastToPROJCharacter OtherActor)
  (Utilities|Array|RemoveIndex _things_on_platform (Utilities|Array|LastIndex _things_on_platform)))

(event Collision|EventActorBeginOverlap
  (params (OtherActor :type Actor%20Object%20Reference))
  (Utilities|Casting|CastToPROJCharacter OtherActor)
  (Utilities|Array|Add (Variables|Default|GetThings%20On%20Platform) 0)
  (CallFunction|CheckSwap))

(fn ConstructionScript)

(fn OnRepThingsonPlatform)

(fn OnRepAmountNeededonPlatform)