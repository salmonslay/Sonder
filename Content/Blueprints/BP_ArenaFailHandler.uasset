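; BP_ArenaFailHandler is a Blueprint for arena failure whose Playerdied event checks the state of the two character types.
; The event finds the first BP_SoulCharacter and BP_ThirdPersonCharacter and tests whether the largest axis of each mesh's relative scale is below 0.5.
; Mesh scale serves as the condition, but the branch leads to no action and the construction script is empty.
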(event Custom|Player%20died
  (bind _outactors (Actor|GetAllActorsOfClass "/Game/Blueprints/BP_SoulCharacter.BP_SoulCharacter_C"))
  (bind _outactors_2 (Actor|GetAllActorsOfClass "/Game/ThirdPerson/Blueprints/BP_ThirdPersonCharacter.BP_ThirdPersonCharacter_C"))
  (if (and (< (Math|Vector|GetMaxElement (Variables|/Script/Engine.SceneComponent|GetRelativeScale3D (Variables|/Script/Engine.Character|GetMesh (Utilities|Array|Get(acopy) _outactors)))) 0.5) (< (Math|Vector|GetMaxElement (Variables|/Script/Engine.SceneComponent|GetRelativeScale3D (Variables|/Script/Engine.Character|GetMesh (Utilities|Array|Get(acopy) _outactors_2)))) 0.5))
    _))

(fn ConstructionScript)