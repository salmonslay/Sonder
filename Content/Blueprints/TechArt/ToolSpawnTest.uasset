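; An editor Scriptable Tool test that spawns a static mesh actor where the user clicks.
; Setup adds a "Settings" spawn property set, which the click logic never reads.
; A click runs a visibility trace, spawning at the hit location or warning when nothing is hit.
; The trace has zero length because the scaled ray direction is unwired, and no mesh is supplied to the spawned actor.
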(event EventOnScriptSetup
  (bind _returnvalue (Class|ScriptableInteractiveTool|AddPropertySetOfType "/Game/Blueprints/TechArt/Spawn_Properties.Spawn_Properties_C" "Settings")
    (:Success
      (Variables|Default|SetNew%20Property%20Set _returnvalue))))

(event EventOnHitbyClick
  (params (ClickPos :type Input%20Device%20Ray%20Structure) (Modifiers :type Scriptable%20Tool%20Modifier%20States%20Structure%20%28by%20ref%29))
  (bind _worldray (Utilities|Struct|BreakInputDeviceRay ClickPos))
  (bind (_origin _direction) (Utilities|Struct|BreakRay _worldray))
  (bind (_outhit _returnvalue) (Collision|LineTraceByChannel _origin (+ _origin "") "TraceTypeQuery1" false 0 "None"))
  (if _returnvalue
    (bind _returnvalue_2 (Game|SpawnActorfromClass "/Script/Engine.StaticMeshActor" (Math|Conversions|ToTransform(Vector) (.Location (Collision|BreakHitResult _outhit))) "Undefined" "MultiplyWithRoot" 0 0))
    (Components|StaticMesh|SetStaticMesh (Variables|/Script/Engine.StaticMeshActor|GetStaticMeshComponent _returnvalue_2) 0)
    (else
      (Class|ScriptableInteractiveTool|DisplayUserWarningMessage "Nothing clicked"))))