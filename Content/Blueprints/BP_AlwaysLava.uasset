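; BP_AlwaysLava is an actor that starts moving along a referenced track's spline five seconds after play begins.
; A timeline scaled by Duration drives position and rotation by spline distance, resuming from the current Alpha.
; With ShouldWaitAtEnd set, it pauses for TimeToStay at either end, then travels back, looping.
; FMOD plays movement and landing sounds through parameters, with a DoOnce preventing restarts until landing.
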(event Custom|LandedSFX
  (bind _fmodaudio (Variables|Default|GetFMODAudio))
  ;[1 1 1] Function for calling Landing SFX
  (Class|FMODAudioComponent|SetParameter (Variables|Default|GetFMODAudio) "boxLanded" 1.0)
  ;[1 1 1] Function for calling Moving SFX
  (Utilities|FlowControl|DoOnce false) ; enters at Reset
)

(event Custom|StartMovingSFX
  (bind _fmodaudio (Variables|Default|GetFMODAudio))
  ;[1 1 1] Function for calling Moving SFX
  (Utilities|FlowControl|DoOnce false
    (:Completed
      (Class|FMODAudioComponent|SetParameter _fmodaudio "boxLanded" 0.0)
      (Class|FMODAudioComponent|SetParameter _fmodaudio "obstacleType" (Math|Conversions|ToFloat(Integer) (Variables|Default|GetdoorType)))
      (Class|FMODAudioComponent|SetTimelinePosition _fmodaudio)
      (Class|FMODAudioComponent|Play _fmodaudio))))

(event Custom|Move
  (bind _timetostay (Variables|Default|GetTimeToStay))
  (bind _trackref (Variables|Default|GetTrackRef))
  (bind _cameraspline (Variables|/Script/PROJ.CameraSpline|GetCameraSpline _trackref))
  (CallFunction|StartMovingSFX)
  (Components|Timeline|SetPlayRate (Variables|Default|GetMoveToEnd) (/ 1.0 (Variables|Default|GetDuration)))
  (bind _output_get (Variables|Default|SetStartOffset (Variables|Default|GetAlpha)))
  (Components|Timeline|SetNewTime (Variables|Default|GetMoveToEnd) _output_get)
  (bind _alpha (Timeline|MoveToEnd Play)
    (:Update
      (Variables|Default|SetAlpha _alpha)
      (Transformation|SetActorLocationAndRotation (Spline|GetLocationatDistanceAlongSpline _cameraspline (Math|Float|Lerp 0.0 (Spline|GetSplineLength _cameraspline) (Variables|Default|GetAlpha)) "World") (Spline|GetRotationatDistanceAlongSpline (Variables|/Script/PROJ.CameraSpline|GetCameraSpline (Variables|Default|GetTrackRef)) (Math|Float|Lerp 0.0 (Spline|GetSplineLength _cameraspline) (Variables|Default|GetAlpha)) "Local")))
    (:Finished
      (CallFunction|LandedSFX)
      (if (Variables|Default|GetShouldWaitAtEnd)
        (if (== (Variables|Default|GetAlpha) 1.0)
          (Utilities|FlowControl|Delay _timetostay)
          (CallFunction|Reverse)
          (elif (== (Variables|Default|GetAlpha) 0.0)
            (Utilities|FlowControl|Delay _timetostay)
            (CallFunction|Move)))))))

(event Custom|Reverse
  (bind _timetostay (Variables|Default|GetTimeToStay))
  (bind _trackref (Variables|Default|GetTrackRef))
  (bind _cameraspline (Variables|/Script/PROJ.CameraSpline|GetCameraSpline _trackref))
  (CallFunction|StartMovingSFX)
  (bind _alpha (Timeline|MoveToEnd Reverse)
    (:Update
      (Variables|Default|SetAlpha _alpha)
      (Transformation|SetActorLocationAndRotation (Spline|GetLocationatDistanceAlongSpline _cameraspline (Math|Float|Lerp 0.0 (Spline|GetSplineLength _cameraspline) (Variables|Default|GetAlpha)) "World") (Spline|GetRotationatDistanceAlongSpline (Variables|/Script/PROJ.CameraSpline|GetCameraSpline (Variables|Default|GetTrackRef)) (Math|Float|Lerp 0.0 (Spline|GetSplineLength _cameraspline) (Variables|Default|GetAlpha)) "Local")))
    (:Finished
      (CallFunction|LandedSFX)
      (if (Variables|Default|GetShouldWaitAtEnd)
        (if (== (Variables|Default|GetAlpha) 1.0)
          (Utilities|FlowControl|Delay _timetostay)
          (CallFunction|Reverse)
          (elif (== (Variables|Default|GetAlpha) 0.0)
            (Utilities|FlowControl|Delay _timetostay)
            (CallFunction|Move)))))))

(event EventBeginPlay
  (Utilities|FlowControl|Delay 5.0)
  (CallFunction|Move))

(fn ConstructionScript)