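; Spline-following moving platform that starts after a delay, driven by pressure plates and other trigger objects.
; A timeline moves it along TrackRef's spline; all plates pressed or a non-empty MoveReverseArray plays it forward, otherwise it reverses.
; It can wait at the end, return and reset its time-based triggers.
; It refreshes its grid's moving-actor calculation on a throttled tick and drives FMOD moving, landing and underwater audio.
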(event Custom|LandedSFX
  (bind _fmodaudio (Variables|Default|GetFMODAudio))
  ;[1 1 1] Function for calling Landing SFX
  (Class|FMODAudioComponent|SetParameter (Variables|Default|GetFMODAudio) "boxLanded" 1.0)
  ;[1 1 1] Function for calling Moving SFX
  (Utilities|FlowControl|DoOnce false) ; enters at Reset
)

(event Custom|StartMovingSFX
  (bind _fmodaudio (Variables|Default|GetFMODAudio))
  ;[1 1 1] Function for calling Moving SFX
  (Utilities|FlowControl|DoOnce false
    (:Completed
      (Class|FMODAudioComponent|SetParameter _fmodaudio "boxLanded" 0.0)
      (Class|FMODAudioComponent|SetParameter _fmodaudio "obstacleType" (Math|Conversions|ToFloat(Integer) (Variables|Default|GetdoorType)))
      (Class|FMODAudioComponent|SetTimelinePosition _fmodaudio)
      (Class|FMODAudioComponent|Play _fmodaudio))))

(event Custom|MultiplePlates
  (bind _platesarepressed (Variables|Default|GetPlatesArePressed))
  (for _array_element (Variables|Default|GetPlateAmountArray)
    (Utilities|Array|Add (Variables|Default|GetPlatesArePressed) (Variables|/Game/Blueprints/PressurePlates/BP_PressurePlateMultiple.BP_PressurePlateMultiple_C|GetIsPressed _array_element)))
  (if (Utilities|Array|ContainsItem _platesarepressed false)
    (Development|PrintString "One false")
    (Class|MovingPlatform|StartReverse)
    (else
      (Development|PrintString "All true")
      (Class|MovingPlatform|StartMoving)))
  (Utilities|Array|Clear _platesarepressed))

(event Custom|MultiMoveReverse
  (if (> (Utilities|Array|Length (Variables|Default|GetMoveReverseArray)) 0)
    (Class|MovingPlatform|StartMoving)
    (else
      (Class|MovingPlatform|StartReverse))))

(event EventBeginPlay
  (bind _currentgrid (Variables|Default|GetCurrentGrid))
  (Utilities|IsValid _currentgrid
    (:Is%20Valid
      (Utilities|FlowControl|Delay 0.2)
      (Class|Grid|CalculateMovingActor _currentgrid self)
      (if (Variables|Default|GetInWater)
        (Class|FMODAudioComponent|SetParameter (Variables|Default|GetFMODAudio) "InWater" 1.0)))))

(event EventTick
  (params (DeltaSeconds :type Float%20%28single-precision%29))
  (bind _currentgrid (Variables|Default|GetCurrentGrid))
  (Utilities|FlowControl|DoOnce false :!label _label
    (:Completed
      (Utilities|IsValid _currentgrid
        (:Is%20Valid
          (Class|Grid|CalculateMovingActor _currentgrid self)
          (Utilities|FlowControl|Delay 0.2)
          (goto _label Reset))))))

(event EventStartMoving
  (bind _trackref (Variables|Default|GetTrackRef))
  (bind _cameraspline (Variables|/Script/PROJ.CameraSpline|GetCameraSpline _trackref))
  (Utilities|FlowControl|Delay (Variables|Default|GetDelayTime))
  (CallFunction|StartMovingSFX)
  (Components|Timeline|SetPlayRate (Variables|Default|GetMoveToEnd) (/ 1.0 (Variables|Default|GetDuration)))
  (bind _output_get (Variables|Default|SetStartOffset (Variables|Default|GetAlpha)))
  (Components|Timeline|SetNewTime (Variables|Default|GetMoveToEnd) _output_get)
  (bind _alpha (Timeline|MoveToEnd Play)
    (:Update
      (Variables|Default|SetAlpha _alpha)
      (Transformation|SetActorLocationAndRotation (Spline|GetLocationatDistanceAlongSpline _cameraspline (Math|Float|Lerp 0.0 (Spline|GetSplineLength _cameraspline) (Variables|Default|GetAlpha)) "World") (Spline|GetRotationatDistanceAlongSpline (Variables|/Script/PROJ.CameraSpline|GetCameraSpline (Variables|Default|GetTrackRef)) (Math|Float|Lerp 0.0 (Spline|GetSplineLength _cameraspline) (Variables|Default|GetAlpha)) "Local")))
    (:Finished
      (CallFunction|LandedSFX)
      (if (Variables|Default|GetShouldWaitAtEnd)
        (if (== (Variables|Default|GetAlpha) 1.0)
          (Utilities|FlowControl|Delay (Variables|Default|GetTimeToStay))
          (Class|MovingPlatform|StartReverse)
          (Utilities|FlowControl|Delay (Variables|Default|GetDuration))
          (for _array_element (Variables|Default|GetMoveReversePlates)
            (bind _asbp_pressure_plate_time_based (Utilities|Casting|CastToBP_PressurePlateTimeBased _array_element)
              (:then
                (Default|ResetObject _asbp_pressure_plate_time_based))
              (:CastFailed
                (bind _asbp_pulse_object_time_based (Utilities|Casting|CastToBP_PulseObjectTimeBased _array_element))
                (Default|ResetObject _asbp_pulse_object_time_based)))))))))

(event EventStartReverse
  (bind _trackref (Variables|Default|GetTrackRef))
  (bind _cameraspline (Variables|/Script/PROJ.CameraSpline|GetCameraSpline _trackref))
  (CallFunction|StartMovingSFX)
  (bind _alpha (Timeline|MoveToEnd Reverse)
    (:Update
      (Variables|Default|SetAlpha _alpha)
      (Transformation|SetActorLocationAndRotation (Spline|GetLocationatDistanceAlongSpline _cameraspline (Math|Float|Lerp 0.0 (Spline|GetSplineLength _cameraspline) (Variables|Default|GetAlpha)) "World") (Spline|GetRotationatDistanceAlongSpline (Variables|/Script/PROJ.CameraSpline|GetCameraSpline (Variables|Default|GetTrackRef)) (Math|Float|Lerp 0.0 (Spline|GetSplineLength _cameraspline) (Variables|Default|GetAlpha)) "Local")))
    (:Finished
      (CallFunction|LandedSFX)
      (if (Variables|Default|GetShouldWaitAtEnd)
        (if (== (Variables|Default|GetAlpha) 1.0)
          (Utilities|FlowControl|Delay (Variables|Default|GetTimeToStay))
          (Class|MovingPlatform|StartReverse)
          (Utilities|FlowControl|Delay (Variables|Default|GetDuration))
          (for _array_element (Variables|Default|GetMoveReversePlates)
            (bind _asbp_pressure_plate_time_based (Utilities|Casting|CastToBP_PressurePlateTimeBased _array_element)
              (:then
                (Default|ResetObject _asbp_pressure_plate_time_based))
              (:CastFailed
                (bind _asbp_pulse_object_time_based (Utilities|Casting|CastToBP_PulseObjectTimeBased _array_element))
                (Default|ResetObject _asbp_pulse_object_time_based)))))))))

(fn ConstructionScript)