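; BP_FreezeConstraintWalls is a trigger actor that moves walls according to how many PROJCharacter actors overlap it.
; Entering characters are added to ThingsInTrigger, and MoveWallsToLoc runs when the count equals AmountNeededInTrigger.
; On exit, the last array entry is removed regardless of who left, and RemoveWallsFromLoc runs while the count is below that threshold.
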(event EventBeginPlay)

(event EventTick
  (params (DeltaSeconds :type Float%20%28single-precision%29)))

(event Collision|EventActorBeginOverlap
  (params (OtherActor :type Actor%20Object%20Reference))
  (bind _things_in_trigger (Variables|Default|GetThings%20In%20Trigger))
  (Utilities|Casting|CastToPROJCharacter OtherActor)
  (Utilities|Array|Add _things_in_trigger 0)
  (if (== (Utilities|Array|Length _things_in_trigger) (Variables|Default|GetAmount%20Needed%20In%20Trigger))
    (Class|FreezeConstraintWalls|MoveWallstoLoc)))

(event Collision|EventActorEndOverlap
  (params (OtherActor :type Actor%20Object%20Reference))
  (bind _things_in_trigger (Variables|Default|GetThings%20In%20Trigger))
  (Utilities|Casting|CastToPROJCharacter OtherActor)
  (Utilities|Array|RemoveIndex _things_in_trigger (Utilities|Array|LastIndex _things_in_trigger))
  (if (< (Utilities|Array|Length _things_in_trigger) (Variables|Default|GetAmount%20Needed%20In%20Trigger))
    (Class|FreezeConstraintWalls|RemoveWallsfromLoc)))

(fn ConstructionScript)