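; BP_EnemyJumpTrigger is a trigger that gates jumps for waiting ShadowCharacter enemies based on the presence of a MovingPlatform.
; An overlapping platform is stored and calls AllowJump; its exit calls DenyJump.
; Entering enemies are added as waiting and exiting ones removed, with the enemy-overlap flag cleared once none remain.
; The jump and waiting-list functions are defined outside this graph, which only routes overlap events.
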(event Collision|EventActorBeginOverlap
  (params (OtherActor :type Actor%20Object%20Reference))
  (bind _asmoving_platform (Utilities|Casting|CastToMovingPlatform OtherActor)
    (:then
      (Variables|Default|SetbIsOverlappingWithMovingPlatform true)
      (Variables|Default|SetOverlappingPlatform _asmoving_platform)
      (Class|EnemyJumpTrigger|AllowJump))
    (:CastFailed
      (bind _asshadow_character (Utilities|Casting|CastToShadowCharacter OtherActor))
      (Variables|Default|SetbIsOverlappingWithEnemy true)
      (Class|EnemyJumpTrigger|AddWaitingEnemy _asshadow_character))))

(event EventTick
  (params (DeltaSeconds :type Float%20%28single-precision%29)))

(event Collision|EventActorEndOverlap
  (params (OtherActor :type Actor%20Object%20Reference))
  (Utilities|Casting|CastToMovingPlatform OtherActor
    (:then
      (Variables|Default|SetbIsOverlappingWithMovingPlatform false)
      (Class|EnemyJumpTrigger|DenyJump))
    (:CastFailed
      (bind _asshadow_character (Utilities|Casting|CastToShadowCharacter OtherActor))
      (Class|EnemyJumpTrigger|RemoveWaitingEnemy _asshadow_character)
      (bind _returnvalue (Class|EnemyJumpTrigger|IsOverlappingwithEnemies))
      (if (not _returnvalue)
        (Variables|Default|SetbIsOverlappingWithEnemy false)))))

(fn ConstructionScript)