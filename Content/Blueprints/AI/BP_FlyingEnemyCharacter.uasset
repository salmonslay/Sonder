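; Flying eye enemy character that adds audio, VFX and lifecycle handling to attack, damage and death events.
; Each event sets an FMOD eye-sound parameter, alongside effects like the charge-up and laser beam.
; Tick updates the health bar widget and animates two dissolve materials for spawn fade-in and death fade-out.
; On death it detaches its controller, leaves its manager on authority, then fills the arena progress bar and destroys itself.
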(event EventOnTakenDamageEvent
  (params (DamageTaken :type Float%20%28single-precision%29))
  ;[1 1 1] Take damage
  (Niagara|SpawnSystematLocation 0 (Transformation|GetActorLocation))
  (bind _returnvalue (Class|FMODBlueprintStatics|PlayEventAttached "/Game/FMOD/Events/SFX/EyeSounds.EyeSounds" (Variables|Default|GetFMODAudio) "None" "0, 0, 0" "KeepRelativeOffset"))
  (Class|FMODAudioComponent|SetParameter _returnvalue "eyeSounds" 4.0)
  (Development|SetHiddeninGame (Variables|Default|GetVFX_ChargeUp) true false))

(event EventTick
  (params (DeltaSeconds :type Float%20%28single-precision%29))
  (Utilities|FlowControl|Sequence
    (:then_0
      ;[1 1 1] Update hp bar
      (bind _asuwbp_enemy_health_bar (Utilities|Casting|CastToUWBP_EnemyHealthBar (UserInterface|GetUserWidgetObject (Variables|Default|GetHealthBarWidget))))
      (Variables|/Game/UI/Gameplay/UWBP_EnemyHealthBar.UWBP_EnemyHealthBar_C|SetFill%20percentage _asuwbp_enemy_health_bar (Class|BaseHealthComponent|GetHealthPercent (Variables|Default|GetEnemyHealthComponent))))
    (:then_1
      (if (Variables|Default|GetFadingOut)
        (bind _output_get (Variables|Default|SetFadeTimer (+ (Variables|Default|GetFadeTimer) DeltaSeconds)))
        (Rendering|Material|SetScalarParameterValue (Variables|Default|GetDMI_White) "Bounds" (+ (* (/ _output_get (Variables|Default|GetFadeInTime)) (- (Variables|Default|GetMaterialBoundsUpperLimit) (Variables|Default|GetMaterialBoundsLowerLimit))) (Variables|Default|GetMaterialBoundsLowerLimit)) :!class /Script/Engine.MaterialInstanceDynamic)
        (Rendering|Material|SetScalarParameterValue (Variables|Default|GetDMI_Black) "Bounds" (+ (* (/ _output_get (Variables|Default|GetFadeInTime)) (- (Variables|Default|GetMaterialBoundsUpperLimit) (Variables|Default|GetMaterialBoundsLowerLimit))) (Variables|Default|GetMaterialBoundsLowerLimit)) :!class /Script/Engine.MaterialInstanceDynamic)
        (elif (Variables|Default|GetFadingIn)
          (bind _output_get_2 (Variables|Default|SetFadeTimer (+ (Variables|Default|GetFadeTimer) DeltaSeconds)))
          (Rendering|Material|SetScalarParameterValue (Variables|Default|GetDMI_White) "Bounds" (- (Variables|Default|GetMaterialBoundsUpperLimit) (* (/ _output_get_2 (Variables|Default|GetFadeInTime)) (- (Variables|Default|GetMaterialBoundsUpperLimit) (Variables|Default|GetMaterialBoundsLowerLimit)))) :!class /Script/Engine.MaterialInstanceDynamic)
          (Rendering|Material|SetScalarParameterValue (Variables|Default|GetDMI_Black) "Bounds" (- (Variables|Default|GetMaterialBoundsUpperLimit) (* (/ _output_get_2 (Variables|Default|GetFadeInTime)) (- (Variables|Default|GetMaterialBoundsUpperLimit) (Variables|Default|GetMaterialBoundsLowerLimit)))) :!class /Script/Engine.MaterialInstanceDynamic))))))

(event EventOnChargingAttackEvent
  (params (ChargingDuration :type Float%20%28single-precision%29))
  ;[1 1 1] Charge attack
  (bind _returnvalue (Class|FMODBlueprintStatics|PlayEventAttached "/Game/FMOD/Events/SFX/EyeSounds.EyeSounds" (Variables|Default|GetFMODAudio) "None" "0, 0, 0" "KeepRelativeOffset"))
  (Class|FMODAudioComponent|SetParameter _returnvalue "eyeSounds" 1.0)
  (Development|SetHiddeninGame (Variables|Default|GetVFX_ChargeUp) false false))

(event EventOnDeathEvent
  (bind _manager (Variables|Default|GetManager))
  (Class|FMODAudioComponent|Stop (Variables|Default|GetFMODAudio))
  (bind _returnvalue (Class|FMODBlueprintStatics|PlayEventAttached "/Game/FMOD/Events/SFX/EyeSounds.EyeSounds" (Variables|Default|GetFMODAudio) "None" "0, 0, 0" "KeepRelativeOffset"))
  (Class|FMODAudioComponent|SetParameter _returnvalue "eyeSounds" 2.0)
  (Class|Pawn|DetachfromControllerPendingDestroy)
  (if (and (== (Networking|GetLocalRole) 3) (Utilities|IsValid _manager))
    (bind _asflying_enemy_character (Utilities|Casting|CastToFlyingEnemyCharacter self))
    (Class|CombatManager|RemoveEnemy _manager _asflying_enemy_character))
  (Variables|Default|SetFadingOut true)
  (Variables|Default|SetFadeTimer 0.0)
  (Utilities|FlowControl|Delay (Variables|Default|GetFadeOutTime))
  (Variables|Default|SetFadingOut false)
  (bind _outactors (Actor|GetAllActorsOfClass "/Game/Blueprints/BP_ArenaProgress.BP_ArenaProgress_C"))
  (if (> (Utilities|Array|Length _outactors) 0)
    (Default|FillBar (Utilities|Array|Get(acopy) _outactors)))
  (Actor|DestroyActor))

(event EventOnPerformAttackEvent
  (params (AttackDuration :type Float%20%28single-precision%29))
  ;[1 1 1] Perform attack
  (bind _returnvalue (Class|FMODBlueprintStatics|PlayEventAttached "/Game/FMOD/Events/SFX/EyeSounds.EyeSounds" (Variables|Default|GetFMODAudio) "None" "0, 0, 0" "KeepRelativeOffset"))
  (Class|FMODAudioComponent|SetParameter _returnvalue "eyeSounds" 0.0)
  (Niagara|SpawnSystematLocation "/Game/Blueprints/AI/LaserBeam.LaserBeam" (Transformation|GetActorLocation) (Transformation|GetActorRotation))
  (Development|SetHiddeninGame (Variables|Default|GetVFX_ChargeUp) true false))

(event EventBeginPlay
  (bind _materialboundsupperlimit (Variables|Default|GetMaterialBoundsUpperLimit))
  (Utilities|FlowControl|Sequence
    (:then_0
      (bind _returnvalue (Class|FMODBlueprintStatics|PlayEventAttached "/Game/FMOD/Events/SFX/EyeSounds.EyeSounds" (Variables|Default|GetFMODAudio) "None" "0, 0, 0" "KeepRelativeOffset"))
      (Class|FMODAudioComponent|SetParameter _returnvalue "eyeSounds" 3.0))
    (:then_1
      ;[1 1 1] Creating, setting, and initializing the dynamic materials
      (bind _returnvalue_2 (Rendering|Material|CreateDynamicMaterialInstance "/Game/VFX/Shaders/Eye_Dissolve/MM_Eye_Dissolve.MM_Eye_Dissolve" "DMI_Eye_Dissolve_White" "None" :!class /Script/Engine.KismetMaterialLibrary))
      (bind _output_get (Variables|Default|SetDMI_White _returnvalue_2))
      (Rendering|Material|SetMaterial (Variables|Character|GetMesh) 0 _output_get)
      (bind _returnvalue_3 (Rendering|Material|CreateDynamicMaterialInstance "/Game/VFX/Shaders/Eye_Dissolve/MM_Eye_Dissolve.MM_Eye_Dissolve" "DMI_Eye_Dissolve_Black" "None" :!class /Script/Engine.KismetMaterialLibrary))
      (bind _output_get_2 (Variables|Default|SetDMI_Black _returnvalue_3))
      (Rendering|Material|SetMaterial (Variables|Character|GetMesh) 1 _output_get_2)
      (Rendering|Material|SetVectorParameterValue (Variables|Default|GetDMI_White) "BaseColor" "(R=1.000000,G=1.000000,B=1.000000,A=1.000000)" :!class /Script/Engine.MaterialInstanceDynamic)
      (Rendering|Material|SetScalarParameterValue (Variables|Default|GetDMI_White) "Bounds" _materialboundsupperlimit :!class /Script/Engine.MaterialInstanceDynamic)
      (Rendering|Material|SetScalarParameterValue (Variables|Default|GetDMI_Black) "Bounds" _materialboundsupperlimit :!class /Script/Engine.MaterialInstanceDynamic)
      (Variables|Default|SetFadingIn true)
      (Variables|Default|SetFadeTimer 0.0)
      (Utilities|FlowControl|Delay (Variables|Default|GetFadeInTime))
      (Variables|Default|SetFadingIn false))))

(fn ConstructionScript)