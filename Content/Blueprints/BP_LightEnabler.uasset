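; BP_LightEnabler is an actor that delays the appearance of level lighting and fog after play begins.
; On BeginPlay it finds the SkyLight, hides it, waits for DelayToEnableLight, then shows each actor's component in the Lights and Fog arrays.
; The SkyLight is shown again inside the Fog loop, so it returns only if that array has entries.
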(event EventBeginPlay
  (bind _returnvalue (Actor|GetActorOfClass "/Script/Engine.SkyLight"))
  (bind _output_get (Variables|Default|SetSkyLight _returnvalue))
  (Rendering|SetVisibility (Variables|/Script/Engine.SkyLight|GetLightComponent _output_get) false false)
  (Utilities|FlowControl|Delay (Variables|Default|GetDelayToEnableLight))
  (for _array_element (Variables|Default|GetLights)
    (Rendering|SetVisibility (Variables|/Script/Engine.Light|GetLightComponent _array_element) true false))
  (for _array_element_2 (Variables|Default|GetFog)
    (Rendering|SetVisibility (Variables|/Script/Engine.ExponentialHeightFog|GetComponent _array_element_2) true false)
    (Rendering|SetVisibility (Variables|/Script/Engine.SkyLight|GetLightComponent (Variables|Default|GetSkyLight)) true false)))

(fn ConstructionScript)