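; An explosion actor that plays a burst of staggered blasts with sound and camera shake when its Explosion event is called.
; The event fires one world camera shake at the actor, then loops through short random delays, each followed by FMOD audio and a Niagara effect at a randomly offset location.
; A DoN node counts the loop up to NumberOfExplosions and is never reset.
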(event Custom|Event%20Explosion
  (bind _returnvalue (Transformation|GetActorLocation))
  (bind _numberofexplosions (Variables|Default|GetNumberOfExplosions))
  (Camera|PlayWorldCameraShake "/Game/LevelSequencers/BPCS_CameraShakeLive.BPCS_CameraShakeLive_C" (Transformation|GetActorLocation) 0.0 5e+03)
  (Utilities|FlowControl|Delay (/ (Math|Random|RandomFloat) 1e+01) :!label _label)
  (Class|FMODAudioComponent|Play (Variables|Default|GetFMODAudio))
  (Niagara|SpawnSystematLocation (Variables|Default|GetNiagaraSystem) (Math|Vector|MakeVector (+ (* (Math|Random|RandomFloatinRange -1.0 1.0) (Variables|Default|GetOffsetX)) (.x _returnvalue)) (+ (* (Math|Random|RandomFloatinRange -1.0 1.0) (Variables|Default|GetOffsetY)) (.y _returnvalue)) (+ (* (Math|Random|RandomFloatinRange -1.0 1.0) (Variables|Default|GetOffsetZ)) (.z _returnvalue))))
  (bind _counter (Utilities|FlowControl|DoN _numberofexplosions)
    (:Exit
      (if (not (>= _counter _numberofexplosions))
        (goto _label)))))

(event EventBeginPlay)

(event Collision|EventActorBeginOverlap
  (params (OtherActor :type Actor%20Object%20Reference)))

(event EventTick
  (params (DeltaSeconds :type Float%20%28single-precision%29)))

(fn ConstructionScript)