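; BP_WarningSpotLights is a trigger actor that fires a one-time spotlight and sound cue once enough PROJCharacters are inside it.
; Overlaps grow and shrink the ThingsInTrigger array, with exits removing the last entry rather than the departing actor.
; When the count equals AmountNeededInTrigger, a DoOnce toggles SpotLight visibility and plays the FMOD event assigned on BeginPlay.
; A trailing one-second retriggerable delay drives nothing further.
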(event EventBeginPlay
  (Class|FMODAudioComponent|SetEvent (Variables|Default|GetFMODAudio) (Variables|Default|GetFMOD%20Event)))

(event Collision|EventActorBeginOverlap
  (params (OtherActor :type Actor%20Object%20Reference))
  (bind _things_in_trigger (Variables|Default|GetThings%20In%20Trigger))
  (Utilities|Casting|CastToPROJCharacter OtherActor)
  (Utilities|Array|Add _things_in_trigger 0)
  (if (== (Utilities|Array|Length _things_in_trigger) (Variables|Default|GetAmount%20Needed%20In%20Trigger))
    (Utilities|FlowControl|DoOnce false
      (:Completed
        (Rendering|ToggleVisibility (Variables|Default|GetSpotLight) false)
        (Class|FMODAudioComponent|Play (Variables|Default|GetFMODAudio))
        (Utilities|FlowControl|RetriggerableDelay 1.0)))))

(event Collision|EventActorEndOverlap
  (params (OtherActor :type Actor%20Object%20Reference))
  (bind _things_in_trigger (Variables|Default|GetThings%20In%20Trigger))
  (Utilities|Casting|CastToPROJCharacter OtherActor)
  (Utilities|Array|RemoveIndex _things_in_trigger (Utilities|Array|LastIndex _things_in_trigger)))

(fn ConstructionScript)