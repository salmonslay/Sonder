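; Trigger actor that ends an endless survival run once two player characters overlap it, flagging each as safe while inside.
; On completion it stops combat and music, then compares the combat manager's score with the leaderboard value queried at BeginPlay.
; A popup reports a new high score or game over.
; Retry server-travels to ArenaSurvival on the host only, while Main menu destroys sessions before opening the menu level.
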(event Custom|RetryEvent
  (|Retry (stale Collision|EventActorBeginOverlap _returnvalue_2)))

(event Custom|GoToMainMenu
  (|MainMenu))

(event EventBeginPlay
  (bind _leaderboardvalue (|LeaderboardQuery (Game|GetPlayerController 0) "endless_endless")
    (:then
      (Input|SetInputModeGameOnly (Game|GetPlayerController 0) false))
    (:OnSuccess
      (Variables|Default|SetLeaderboard%20Value _leaderboardvalue))))

(event Collision|EventActorBeginOverlap
  (params (OtherActor :type Actor%20Object%20Reference))
  (bind _returnvalue (Game|GetPlayerController 0))
  (bind _overlapping_actors (Variables|Default|GetOverlapping%20Actors))
  (bind _asprojcharacter (Utilities|Casting|CastToPROJCharacter OtherActor))
  (Variables|/Script/Sonder.PROJCharacter|SetbIsSafe _asprojcharacter true)
  (Utilities|Array|AddUnique _overlapping_actors OtherActor)
  (if (>= (Utilities|Array|Length _overlapping_actors) 2)
    (bind _outactors (Actor|GetAllActorsOfClass "/Game/Blueprints/Spawning/BP_CombatManager.BP_CombatManager_C"))
    (Development|PrintString (Utilities|String|ToString(Integer) (Variables|Default|GetLeaderboard%20Value)))
    (Variables|Default|SetTotal%20Score (Variables|/Script/Sonder.CombatManager|GetTotalScore (Utilities|Array|Get(acopy) _outactors)))
    (Class|CombatManager|EndCombat (Utilities|Array|Get(acopy) _outactors))
    (Class|FMODAudioComponent|Stop (Variables|/Script/FMODStudio.FMODAmbientSound|GetAudioComponent (Variables|Default|GetEndlessOSTFmod)))
    (Utilities|FlowControl|Delay 0.5)
    (bind _returnvalue_2 (UserInterface|CreateWidget "/Game/UI/Menu/UWBP_Popup.UWBP_Popup_C" (Game|GetPlayerController 0) (select (> (Variables|Default|GetTotal%20Score) (Variables|Default|GetLeaderboard%20Value)) "NewHigh" "GameOver") (select (> (Variables|Default|GetTotal%20Score) (Variables|Default|GetLeaderboard%20Value)) (Utilities|Text|FormatText "EndlessScoreNoHigh" (Variables|Default|GetTotal%20Score)) (Utilities|Text|FormatText "EndlessScoreWithHigh" (Variables|Default|GetTotal%20Score) (Variables|Default|GetLeaderboard%20Value))) (select (Ability|HasAuthority) "Retry" "MenuWaitingForHost") "Main menu" true))
    (UserInterface|Viewport|AddtoViewport _returnvalue_2 0)
    (Input|SetInputModeUIOnly _returnvalue _returnvalue_2 "DoNotLock" false)
    (Variables|/Script/Engine.PlayerController|SetbShowMouseCursor _returnvalue true)
    (EventDispatchers|BindEventtoButton1Clicked _returnvalue_2 (delegate Custom|RetryEvent))
    (EventDispatchers|BindEventtoButton2Clicked _returnvalue_2 (delegate Custom|GoToMainMenu))))

(event Collision|EventActorEndOverlap
  (params (OtherActor :type Actor%20Object%20Reference))
  (Utilities|Array|RemoveItem (Variables|Default|GetOverlapping%20Actors) OtherActor)
  (bind _asprojcharacter (Utilities|Casting|CastToPROJCharacter OtherActor))
  (Variables|/Script/Sonder.PROJCharacter|SetbIsSafe _asprojcharacter false))

(fn ConstructionScript)