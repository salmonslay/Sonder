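; BP_SonderGameInstance is the game instance that handles online session invites and opens the Steam user overlay.
; Accepting an invite disables join actions on top-level main menu widgets, then joins the session, flagging IsCurrentlyJoining on success or re-enabling those actions on failure.
; Received invites only print a message, and CreateSession is an empty event.
; An unconnected chain that would swap the main menu for a lobby widget never runs.
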(event Custom|CreateSession%20💻)

(event Custom|OpenOverlay
  (Class|AdvancedSteamFriendsLibrary|OpenSteamUserOverlay :DialogType "steamid"))

(event EventOnSessionInviteAccepted
  (params (LocalPlayerNum :type Integer) (PersonInvited :type BP%20Unique%20Net%20Id%20Structure) (SessionToJoin :type Blueprint%20Session%20Result%20Structure%20%28by%20ref%29))
  (CallFunction|ToggleJoinActions false "SOFIA: Accepted game invite")
  (|JoinSession (Game|GetPlayerController 0) SessionToJoin
    (:OnSuccess
      (Variables|Default|SetbIsCurrentlyJoining true))
    (:OnFailure
      (CallFunction|ToggleJoinActions true "SOFIA: Could not join session from accepted invite"))))

(event EventOnSessionInviteReceived
  (params (LocalPlayerNum :type Integer) (PersonInviting :type BP%20Unique%20Net%20Id%20Structure) (AppId :type String) (SessionToJoin :type Blueprint%20Session%20Result%20Structure%20%28by%20ref%29))
  (Development|PrintString "You recieved an invite "))

(fn ToggleJoinActions
  (params (Enable :type Boolean) (Print%20message :type String))
  (bind _foundwidgets (Widget|GetAllWidgetsOfClass "/Game/UI/Menu/UWBP_MainMenu.UWBP_MainMenu_C" true))
  (for _array_element _foundwidgets
    (Default|ToggleJoinActions _array_element Enable Print%20message)))