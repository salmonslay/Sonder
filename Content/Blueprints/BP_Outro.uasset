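; BP_Outro is an actor that runs the game's ending sequence when play begins.
; It marks the Ending and Arena2 levels completed in the save game, then waits on a fixed timer before showing the credits widget.
; After a second delay it destroys the online session and, once that succeeds, opens the main menu level.
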(event EventBeginPlay
  (Variables|Default|SetSave (Class|PROJCharacter|GetSaveGameSafe))
  (Class|SonderSaveGame|AddLevelCompleted (Variables|Default|GetSave) "Ending")
  (Class|SonderSaveGame|AddLevelCompleted (Variables|Default|GetSave) "Arena2")
  (Class|PROJCharacter|SetSaveGame (Variables|Default|GetSave))
  (Utilities|FlowControl|Delay 37.5)
  (bind _returnvalue (UserInterface|CreateWidget "/Game/UI/Menu/UWBP_Credits.UWBP_Credits_C"))
  (UserInterface|Viewport|AddtoViewport _returnvalue 0)
  (Utilities|FlowControl|Delay 14.5)
  (|DestroySession (Game|GetPlayerController 0)
    (:then
      (Game|OpenLevel(byObjectReference) "/Game/Maps/MainMenu.MainMenu"))))

(event Collision|EventActorBeginOverlap
  (params (OtherActor :type Actor%20Object%20Reference)))

(event EventTick
  (params (DeltaSeconds :type Float%20%28single-precision%29)))

(fn ConstructionScript)