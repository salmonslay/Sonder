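; Level exit trigger that moves the game to another level once at least two actors overlap it.
; Characters inside are flagged safe until they leave.
; Reaching the count marks the configured level as completed in the save game and starts a one-time screen fade widget.
; When the fade finishes, the authority performs a server travel to the target level.
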(event Custom|Server%20travel
  (if (Ability|HasAuthority)
    (Class|AdvancedSessionsLibrary|ServerTravel (Variables|Default|GetLevel%20name) false false)))

(event EventBeginPlay)

(event Collision|EventActorBeginOverlap
  (params (OtherActor :type Actor%20Object%20Reference))
  (bind _returnvalue (Class|PROJCharacter|GetSaveGameSafe))
  (bind _overlapping_actors (Variables|Default|GetOverlapping%20actors))
  (bind _asprojcharacter (Utilities|Casting|CastToPROJCharacter OtherActor))
  (Variables|/Script/PROJ.PROJCharacter|SetbIsSafe _asprojcharacter true)
  (Utilities|Array|AddUnique _overlapping_actors OtherActor)
  (if (and (>= (Utilities|Array|Length _overlapping_actors) 2) (not (Variables|Default|GetIs%20switching?)))
    (Class|SonderSaveGame|AddLevelCompleted _returnvalue (Variables|Default|GetLevel%20to%20mark%20as%20finished))
    (Class|PROJCharacter|SetSaveGame _returnvalue)
    (Variables|Default|SetIs%20switching? true)
    (bind _returnvalue_2 (UserInterface|CreateWidget "/Game/UI/Menu/UWBP_SceneFade.UWBP_SceneFade_C"))
    (UserInterface|Viewport|AddtoViewport _returnvalue_2 0)
    (EventDispatchers|AssignDoneFading _returnvalue_2 (delegate Custom|Server%20travel))))

(event Collision|EventActorEndOverlap
  (params (OtherActor :type Actor%20Object%20Reference))
  (Utilities|Array|RemoveItem (Variables|Default|GetOverlapping%20actors) OtherActor)
  (bind _asprojcharacter (Utilities|Casting|CastToPROJCharacter OtherActor))
  (Variables|/Script/PROJ.PROJCharacter|SetbIsSafe _asprojcharacter false))

(fn ConstructionScript)