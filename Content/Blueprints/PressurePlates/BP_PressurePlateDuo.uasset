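; Pressure plate that works jointly with every other plate of its class, playing a cutscene and checking the speedrun achievement once all are pressed.
; Character overlaps, or StartMove when grenade triggering is allowed, add to an occupant count that sets the pressed state at a threshold.
; State changes animate the button and play a parameterized sound event.
; IsRight and the triggering character's class select which cutscene plays through a server RPC.
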(event OnComponentBeginOverlap(TriggerArea)
  (params (OverlappedComponent :type Primitive%20Component%20Object%20Reference) (OtherActor :type Actor%20Object%20Reference) (OtherComp :type Primitive%20Component%20Object%20Reference) (OtherBodyIndex :type Integer) (bFromSweep :type Boolean) (SweepResult :type Hit%20Result%20Structure%20%28by%20ref%29))
  (Utilities|Casting|CastToPROJCharacter OtherActor)
  (CallFunction|MoveEvent))

(event OnComponentEndOverlap(TriggerArea)
  (params (OverlappedComponent :type Primitive%20Component%20Object%20Reference) (OtherActor :type Actor%20Object%20Reference) (OtherComp :type Primitive%20Component%20Object%20Reference) (OtherBodyIndex :type Integer))
  (Utilities|Casting|CastToPROJCharacter OtherActor)
  (Class|PressurePlateBase|StartReverse))

(event Custom|PlayCutscene
  (bind _cutscenes (Variables|Default|GetCutscenes))
  (bind _plates_are_pressed (Variables|Default|GetPlates%20Are%20Pressed))
  (bind _outactors (Actor|GetAllActorsOfClass "BP_PressurePlateDuo_C"))
  (for _array_element _outactors
    (Utilities|Array|Add (Variables|Default|GetPlates%20Are%20Pressed) (Variables|BP_PressurePlateDuo_C|GetIsPressed _array_element)))
  (if (Utilities|Array|ContainsItem _plates_are_pressed false)
    (Utilities|Array|Clear _plates_are_pressed)
    (else
      (Utilities|Casting|CastToBP_ThirdPersonCharacter (stale OnComponentBeginOverlap(TriggerArea) OtherActor)
        (:then
          (if (Variables|Default|GetIsRight)
            (Class|CutsceneManager|ServerRPCPlayCutscene (Utilities|Array|Get(acopy) _cutscenes 1) :!label _label)
            (else
              (Class|CutsceneManager|ServerRPCPlayCutscene (Utilities|Array|Get(acopy) _cutscenes) :!label _label_2))))
        (:CastFailed
          (if (Variables|Default|GetIsRight)
            (goto _label_2)
            (else
              (goto _label)))))
      ;[1 1 1] Try grant speedrun achievement
      (Default|CheckSpeedrun (.AsBP%20Sonder%20Game%20Instance (Utilities|Casting|CastToBP_SonderGameInstance (Game|GetGameInstance)))))))

(event Custom|Move%20Event
  (bind _things_on_platform (Variables|Default|GetThings%20On%20Platform))
  (Utilities|Array|Add _things_on_platform 0)
  (if (>= (Utilities|Array|Length _things_on_platform) (Variables|Default|GetAmountNeededOnPlatform))
    (if (not (Variables|Default|GetIsPressed))
      (Variables|Default|SetIsPressed true)
      (CallFunction|PlayCutscene)
      (bind _returnvalue (Class|FMODBlueprintStatics|PlayEventatLocation "/Game/FMOD/Events/SFX/PressurePlate.PressurePlate" (Math|Conversions|ToTransform(Vector) (Transformation|GetWorldLocation (Variables|Default|GetSM_pressurePlateButton)))))
      (Class|FMODBlueprintStatics|EventInstanceSetParameter _returnvalue "PressureActivated" 0.0)
      ;[1 1 1] Make button pressed
      (Components|Timeline|SetPlayRate (Variables|Default|GetMoveButton) (/ 1.0 0.1))
      (bind _alpha (Timeline|MoveButton Play)
        (:Update
          (Transformation|SetRelativeLocation (Variables|Default|GetSM_pressurePlateButton) (Math|Vector|MakeVector 0.0 0.0 (* _alpha -2.0)) false false))))))

(event EventBeginPlay)

(event Collision|EventActorBeginOverlap
  (params (OtherActor :type Actor%20Object%20Reference)))

(event EventTick
  (params (DeltaSeconds :type Float%20%28single-precision%29)))

(event EventStartMove
  (if (Variables|Default|GetCan%20Be%20Triggered%20By%20Granade)
    (CallFunction|MoveEvent)))

(event EventStartReverse
  (bind _things_on_platform (Variables|Default|GetThings%20On%20Platform))
  (Utilities|Array|RemoveIndex _things_on_platform (Utilities|Array|LastIndex _things_on_platform))
  (if (< (Utilities|Array|Length _things_on_platform) (Variables|Default|GetAmountNeededOnPlatform))
    (Variables|Default|SetIsPressed false)
    (bind _returnvalue (Class|FMODBlueprintStatics|PlayEventatLocation "/Game/FMOD/Events/SFX/PressurePlate.PressurePlate" (Math|Conversions|ToTransform(Vector) (Transformation|GetWorldLocation (Variables|Default|GetSM_pressurePlateButton)))))
    (Class|FMODBlueprintStatics|EventInstanceSetParameter _returnvalue "PressureActivated" 1.0)
    ;[1 1 1] Make button depressed
    (Components|Timeline|SetPlayRate (Variables|Default|GetMoveButton1) (/ 1.0 0.1))
    (bind _alpha (Timeline|MoveButton1 Play)
      (:Update
        (Transformation|SetRelativeLocation (Variables|Default|GetSM_pressurePlateButton) (Math|Vector|MakeVector 0.0 0.0 (* _alpha 5.0)) false false)))))

(fn ConstructionScript)

(fn OnRepThingsonPlatform)