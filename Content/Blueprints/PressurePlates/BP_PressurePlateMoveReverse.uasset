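; Pressure plate that drives a linked moving platform when characters, move boxes or trigger-capable light grenades overlap it.
; Overlaps add or remove entries in its occupant count and the platform's MoveReverseArray, calling MultiMoveReverse around the required threshold.
; Timelines shift the button mesh, and a positional sound event takes a parameter for press or release.
; Grenade exits skip the CanTrigger check, and any exit below threshold calls MultiMoveReverse, even if unpressed.
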(event OnComponentBeginOverlap(TriggerArea)
  (params (OverlappedComponent :type Primitive%20Component%20Object%20Reference) (OtherActor :type Actor%20Object%20Reference) (OtherComp :type Primitive%20Component%20Object%20Reference) (OtherBodyIndex :type Integer) (bFromSweep :type Boolean) (SweepResult :type Hit%20Result%20Structure%20%28by%20ref%29))
  (Utilities|Casting|CastToPROJCharacter OtherActor
    (:then
      (Class|PressurePlateBase|StartMove :!label _label))
    (:CastFailed
      (Utilities|Casting|CastToBP_MoveBox OtherActor
        (:then
          (goto _label))
        (:CastFailed
          (bind _aslight_grenade (Utilities|Casting|CastToLightGrenade (Components|GetOwner OtherComp)))
          (if (Variables|/Script/Sonder.LightGrenade|GetbCanTrigger _aslight_grenade)
            (goto _label)))))))

(event OnComponentEndOverlap(TriggerArea)
  (params (OverlappedComponent :type Primitive%20Component%20Object%20Reference) (OtherActor :type Actor%20Object%20Reference) (OtherComp :type Primitive%20Component%20Object%20Reference) (OtherBodyIndex :type Integer))
  (Utilities|Casting|CastToPROJCharacter OtherActor
    (:then
      _)
    (:CastFailed
      (Utilities|Casting|CastToBP_MoveBox OtherActor
        (:then
          _)
        (:CastFailed
          (Utilities|Casting|CastToLightGrenade (Components|GetOwner OtherComp))))))
  (Class|PressurePlateBase|StartReverse))

(event EventBeginPlay)

(event Collision|EventActorBeginOverlap
  (params (OtherActor :type Actor%20Object%20Reference)))

(event EventStartMove
  (bind _platformtomove (Variables|Default|GetPlatformToMove))
  (bind _things_on_platform (Variables|Default|GetThings%20On%20Platform))
  (Utilities|Array|Add (Variables|/Game/Blueprints/BP_MovingPlatform.BP_MovingPlatform_C|GetMoveReverseArray _platformtomove) 1)
  (Utilities|Array|Add _things_on_platform 0)
  (if (>= (Utilities|Array|Length _things_on_platform) (Variables|Default|GetAmountNeededOnPlatform))
    (if (not (Variables|Default|GetIsPressed))
      (Default|MultiMoveReverse _platformtomove)
      (Variables|Default|SetIsPressed true)
      (bind _returnvalue (Class|FMODBlueprintStatics|PlayEventatLocation "/Game/FMOD/Events/SFX/PressurePlate.PressurePlate" (Math|Conversions|ToTransform(Vector) (Transformation|GetWorldLocation (Variables|Default|GetSM_pressurePlateButton)))))
      (Class|FMODBlueprintStatics|EventInstanceSetParameter _returnvalue "PressureActivated" 0.0)
      ;[1 1 1] Make button pressed
      (Components|Timeline|SetPlayRate (Variables|Default|GetMoveButton) (/ 1.0 0.1))
      (bind _alpha (Timeline|MoveButton Play)
        (:Update
          (Transformation|SetRelativeLocation (Variables|Default|GetSM_pressurePlateButton) (Math|Vector|MakeVector 0.0 0.0 (* _alpha -2.0)) false false))))))

(event EventStartReverse
  (bind _platformtomove (Variables|Default|GetPlatformToMove))
  (bind _things_on_platform (Variables|Default|GetThings%20On%20Platform))
  (bind _movereversearray (Variables|/Game/Blueprints/BP_MovingPlatform.BP_MovingPlatform_C|GetMoveReverseArray _platformtomove))
  (Utilities|Array|RemoveIndex _movereversearray (Utilities|Array|LastIndex _movereversearray))
  (Utilities|Array|RemoveIndex _things_on_platform (Utilities|Array|LastIndex _things_on_platform))
  (if (< (Utilities|Array|Length _things_on_platform) (Variables|Default|GetAmountNeededOnPlatform))
    (Default|MultiMoveReverse _platformtomove)
    (Variables|Default|SetIsPressed false)
    (bind _returnvalue (Class|FMODBlueprintStatics|PlayEventatLocation "/Game/FMOD/Events/SFX/PressurePlate.PressurePlate" (Math|Conversions|ToTransform(Vector) (Transformation|GetWorldLocation (Variables|Default|GetSM_pressurePlateButton)))))
    (Class|FMODBlueprintStatics|EventInstanceSetParameter _returnvalue "PressureActivated" 1.0)
    ;[1 1 1] Make button depressed
    (Components|Timeline|SetPlayRate (Variables|Default|GetMoveButton1) (/ 1.0 0.1))
    (bind _alpha (Timeline|MoveButton1 Play)
      (:Update
        (Transformation|SetRelativeLocation (Variables|Default|GetSM_pressurePlateButton) (Math|Vector|MakeVector 0.0 0.0 (* _alpha 5.0)) false false)))))

(fn ConstructionScript)

(fn OnRepThingsonPlatform)