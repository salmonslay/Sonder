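; Timed pressure plate that starts a linked moving platform when an actor tagged Player steps on it.
; On overlap it deactivates, lowers the button by timeline and plays an attached ticking audio event.
; After a delay covering twice the platform's move duration plus its stay time, it raises the button, re-arms and stops the ticking.
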(event OnComponentBeginOverlap(TriggerArea)
  (params (OverlappedComponent :type Primitive%20Component%20Object%20Reference) (OtherActor :type Actor%20Object%20Reference) (OtherComp :type Primitive%20Component%20Object%20Reference) (OtherBodyIndex :type Integer) (bFromSweep :type Boolean) (SweepResult :type Hit%20Result%20Structure%20%28by%20ref%29))
  (if (Actor|ActorHasTag OtherActor "Player")
    (if (Variables|Default|GetIsActive)
      (Variables|Default|SetIsActive false)
      (Variables|Default|SetIsReset false)
      (Class|PressurePlateBase|StartMove))))

(event Custom|Press%20Plate
  (bind _platformtomove (Variables|Default|GetPlatformToMove))
  (bind _duration (Variables|/Game/Blueprints/BP_MovingPlatform.BP_MovingPlatform_C|GetDuration _platformtomove))
  (Class|MovingPlatform|StartMoving _platformtomove)
  (bind _returnvalue (Class|FMODBlueprintStatics|PlayEventAttached "/Game/FMOD/Events/SFX/WaitTick.WaitTick" (Variables|Default|GetSM_pressurePlateButton) "None" "0, 0, 0" "KeepRelativeOffset"))
  (Utilities|FlowControl|Delay (+ _duration _duration (Variables|/Game/Blueprints/BP_MovingPlatform.BP_MovingPlatform_C|GetTimeToStay _platformtomove)))
  (CallFunction|ResetObject)
  (Class|FMODAudioComponent|Stop _returnvalue))

(event Custom|ResetObject
  (if (not (Variables|Default|GetIsReset))
    (Variables|Default|SetIsActive true)
    (Variables|Default|SetIsReset true)
    ;[1 1 1] Make button depressed
    (Components|Timeline|SetPlayRate (Variables|Default|GetMoveButtonUp) (/ 1.0 0.1))
    (bind _alpha (Timeline|MoveButtonUp Play)
      (:Update
        (Transformation|SetRelativeLocation (Variables|Default|GetSM_pressurePlateButton) (Math|Vector|MakeVector 0.0 0.0 (* _alpha 5.0)) false false)))))

(event EventBeginPlay)

(event Collision|EventActorBeginOverlap
  (params (OtherActor :type Actor%20Object%20Reference)))

(event EventTick
  (params (DeltaSeconds :type Float%20%28single-precision%29)))

(event EventStartMove
  (CallFunction|PressPlate)
  ;[1 1 1] Make button pressed
  (Components|Timeline|SetPlayRate (Variables|Default|GetMoveButtonDown) (/ 1.0 0.1))
  (bind _alpha (Timeline|MoveButtonDown Play)
    (:Update
      (Transformation|SetRelativeLocation (Variables|Default|GetSM_pressurePlateButton) (Math|Vector|MakeVector 0.0 0.0 (* _alpha -2.0)) false false))))

(fn ConstructionScript)