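; BP_PressurePlateBoss is a one-shot pressure plate that triggers a linked explosion when one or two players stand on it, depending on NeedTwoPlayers.
; Overlap events track Player-tagged actors in ThingsOnPlatform.
; Reaching the required count calls EventExplosion on ExplosionToBoom, latches IsPressed and lowers the button mesh through the MoveButton timeline.
; Leaving removes the actor from the list but never releases the plate.
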(event EventBeginPlay
  (if (Variables|Default|GetNeedTwoPlayers)
    (Variables|Default|SetAmount%20Needed%20on%20Platform 2)
    (else
      (Variables|Default|SetAmount%20Needed%20on%20Platform 1))))

(event Collision|EventActorBeginOverlap
  (params (OtherActor :type Actor%20Object%20Reference))
  (bind _things_on_platform (Variables|Default|GetThings%20On%20Platform))
  (if (Actor|ActorHasTag OtherActor "Player")
    (if (not (Variables|Default|GetIsPressed))
      (Utilities|Array|Add _things_on_platform 0)
      (if (== (Utilities|Array|Length _things_on_platform) (Variables|Default|GetAmount%20Needed%20on%20Platform))
        (Class|PressurePlateBase|StartMove)))))

(event Collision|EventActorEndOverlap
  (params (OtherActor :type Actor%20Object%20Reference))
  (bind _things_on_platform (Variables|Default|GetThings%20On%20Platform))
  (if (Actor|ActorHasTag OtherActor "Player")
    (Utilities|Array|RemoveItem _things_on_platform 0)
    (if (< (Utilities|Array|Length _things_on_platform) (Variables|Default|GetAmount%20Needed%20on%20Platform))
      _)))

(event EventStartMove
  (Default|EventExplosion (Variables|Default|GetExplosionToBoom))
  (Variables|Default|SetIsPressed true)
  (bind _alpha (Timeline|MoveButton Play)
    (:Update
      (Transformation|SetRelativeLocation (Variables|Default|GetSM_pressurePlateButton) (Math|Vector|MakeVector 0.0 0.0 (* _alpha -2.0)) false false))))

(fn ConstructionScript)