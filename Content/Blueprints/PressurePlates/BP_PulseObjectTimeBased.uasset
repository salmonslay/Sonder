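; Time-based pulse object that runs a linked platform through a timed move-and-return cycle when its MovePlate event is called.
; While active, MovePlate locks itself, starts PlatformToMove and toggles the RectLight.
; After a delay derived from the platform's travel and stay times, it re-arms, calls StartReverse and toggles the light again.
; Tick prints the active state every frame as debug output.
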(event Custom|MovePlate
  (bind _platformtomove (Variables|Default|GetPlatformToMove))
  (bind _duration (Variables|/Game/Blueprints/BP_MovingPlatform.BP_MovingPlatform_C|GetDuration _platformtomove))
  (if (Variables|Default|GetIsActive)
    (Variables|Default|SetIsActive false)
    (Class|MovingPlatform|StartMoving _platformtomove)
    (Rendering|ToggleVisibility (Variables|Default|GetRectLight) false)
    (Utilities|FlowControl|Delay (+ _duration _duration (Variables|/Game/Blueprints/BP_MovingPlatform.BP_MovingPlatform_C|GetTimeToStay _platformtomove)))
    (Variables|Default|SetIsActive true)
    (Class|MovingPlatform|StartReverse _platformtomove)
    (Rendering|ToggleVisibility (Variables|Default|GetRectLight) false)))

(event EventBeginPlay)

(event Collision|EventActorBeginOverlap
  (params (OtherActor :type Actor%20Object%20Reference)))

(event EventTick
  (params (DeltaSeconds :type Float%20%28single-precision%29))
  (Development|PrintString (Utilities|String|ToString(Boolean) (Variables|Default|GetIsActive))))

(fn ConstructionScript)