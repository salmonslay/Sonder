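; BP_SoulMatActivator is a trigger actor that calls one of the soul character's Mat functions when that character overlaps it.
; On begin overlap, it filters for the "Soul" tag and casts the other actor to BP_SoulCharacter.
; Its MatNr variable selects Mat0, Mat1 or Mat2, with Mat2 as the fallback for any other value.
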(event Collision|EventActorBeginOverlap
  (params (OtherActor :type Actor%20Object%20Reference))
  (if (Actor|ActorHasTag OtherActor "Soul")
    (bind _asbp_soul_character (Utilities|Casting|CastToBP_SoulCharacter OtherActor))
    (if (== (Variables|Default|GetMatNr) 0)
      (Default|Mat0 _asbp_soul_character)
      (elif (== (Variables|Default|GetMatNr) 1)
        (Default|Mat1 _asbp_soul_character)
        (else
          (Default|Mat2 _asbp_soul_character))))))

(fn ConstructionScript)