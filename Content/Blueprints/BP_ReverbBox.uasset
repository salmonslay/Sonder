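; Reverb zone actor that switches FMOD environment snapshots between inside, outside and cave as its box is overlapped.
; Overlap stops all instances of the three snapshots, sets the global EnvironmentIntensity parameter to ReverbStrength and plays the snapshot selected by ReverbType.
; A box flagged FirstBox applies its settings at BeginPlay.
; Overlaps are not filtered by actor, and Tick reads the parameter without using it.
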(event OnComponentBeginOverlap(Box)
  (params (OverlappedComponent :type Primitive%20Component%20Object%20Reference) (OtherActor :type Actor%20Object%20Reference) (OtherComp :type Primitive%20Component%20Object%20Reference) (OtherBodyIndex :type Integer) (bFromSweep :type Boolean) (SweepResult :type Hit%20Result%20Structure%20%28by%20ref%29))
  (bind _returnvalue (Class|FMODBlueprintStatics|FindEventInstances (Variables|Default|GetsnapshotInside)))
  (for _array_element _returnvalue
    (Class|FMODBlueprintStatics|EventInstanceStop _array_element false))
  (bind _returnvalue_2 (Class|FMODBlueprintStatics|FindEventInstances (Variables|Default|GetsnapshotOutside)))
  (for _array_element_2 _returnvalue_2
    (Class|FMODBlueprintStatics|EventInstanceStop _array_element_2 false))
  (bind _returnvalue_3 (Class|FMODBlueprintStatics|FindEventInstances (Variables|Default|GetsnapshotCave)))
  (for _array_element_3 _returnvalue_3
    (Class|FMODBlueprintStatics|EventInstanceStop _array_element_3 false))
  (Class|FMODBlueprintStatics|SetGlobalParameterbyName "EnvironmentIntensity" (Variables|Default|GetreverbStrength))
  (if (== (Variables|Default|GetreverbType) 0.0)
    (Class|FMODBlueprintStatics|PlayEvent2D (Variables|Default|GetsnapshotInside))
    (elif (== (Variables|Default|GetreverbType) 1.0)
      (Class|FMODBlueprintStatics|PlayEvent2D (Variables|Default|GetsnapshotOutside))
      (elif (== (Variables|Default|GetreverbType) 2.0)
        (Class|FMODBlueprintStatics|PlayEvent2D (Variables|Default|GetsnapshotCave))))))

(event EventBeginPlay
  (if (Variables|Default|GetfirstBox)
    (Class|FMODBlueprintStatics|SetGlobalParameterbyName "EnvironmentIntensity" (Variables|Default|GetreverbStrength))
    (if (== (Variables|Default|GetreverbType) 0.0)
      (Class|FMODBlueprintStatics|PlayEvent2D (Variables|Default|GetsnapshotInside))
      (elif (== (Variables|Default|GetreverbType) 1.0)
        (Class|FMODBlueprintStatics|PlayEvent2D (Variables|Default|GetsnapshotOutside))
        (elif (== (Variables|Default|GetreverbType) 2.0)
          (Class|FMODBlueprintStatics|PlayEvent2D (Variables|Default|GetsnapshotCave)))))))

(event Collision|EventActorBeginOverlap
  (params (OtherActor :type Actor%20Object%20Reference)))

(event EventTick
  (params (DeltaSeconds :type Float%20%28single-precision%29))
  (Class|FMODBlueprintStatics|GetGlobalParameterbyName "EnvironmentIntensity"))

(fn ConstructionScript)