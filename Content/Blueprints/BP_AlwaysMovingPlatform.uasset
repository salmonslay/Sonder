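; Platform that moves along a track's spline, starting by itself after a delay when flagged as lava, or via TriggerMovement.
; A timeline scaled by duration sets its position and rotation along the spline, optionally pausing at each end to ping-pong.
; FMOD parameters drive moving and landing sounds, with a DoOnce preventing retriggers until landing.
; Tick uses a DoOnce and delay to periodically have the current grid recalculate this moving actor.
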(event Custom|LandedSFX
  (bind _fmodaudio (Variables|Default|GetFMODAudio))
  ;[1 1 1] Function for calling Landing SFX
  (Class|FMODAudioComponent|SetParameter (Variables|Default|GetFMODAudio) "boxLanded" 1.0)
  ;[1 1 1] Function for calling Moving SFX
  (Utilities|FlowControl|DoOnce false) ; enters at Reset
)

(event Custom|StartMovingSFX
  (bind _fmodaudio (Variables|Default|GetFMODAudio))
  ;[1 1 1] Function for calling Moving SFX
  (Utilities|FlowControl|DoOnce false
    (:Completed
      (Class|FMODAudioComponent|SetParameter _fmodaudio "boxLanded" 0.0)
      (Class|FMODAudioComponent|SetParameter _fmodaudio "obstacleType" (Math|Conversions|ToFloat(Integer) (Variables|Default|GetdoorType)))
      (Class|FMODAudioComponent|SetTimelinePosition _fmodaudio)
      (Class|FMODAudioComponent|Play _fmodaudio))))

(event Custom|TriggerMovement
  (CallFunction|Move))

(event Custom|Move
  (bind _timetostay (Variables|Default|GetTimeToStay))
  (bind _trackref (Variables|Default|GetTrackRef))
  (bind _cameraspline (Variables|/Script/PROJ.CameraSpline|GetCameraSpline _trackref))
  (CallFunction|StartMovingSFX)
  (Components|Timeline|SetPlayRate (Variables|Default|GetMoveToEnd) (/ 1.0 (Variables|Default|GetDuration)))
  (bind _output_get (Variables|Default|SetStartOffset (Variables|Default|GetAlpha)))
  (Components|Timeline|SetNewTime (Variables|Default|GetMoveToEnd) _output_get)
  (bind _alpha (Timeline|MoveToEnd Play)
    (:Update
      (Variables|Default|SetAlpha _alpha)
      (Transformation|SetActorLocationAndRotation (Spline|GetLocationatDistanceAlongSpline _cameraspline (Math|Float|Lerp 0.0 (Spline|GetSplineLength _cameraspline) (Variables|Default|GetAlpha)) "World") (Spline|GetRotationatDistanceAlongSpline (Variables|/Script/PROJ.CameraSpline|GetCameraSpline (Variables|Default|GetTrackRef)) (Math|Float|Lerp 0.0 (Spline|GetSplineLength _cameraspline) (Variables|Default|GetAlpha)) "Local")))
    (:Finished
      (CallFunction|LandedSFX)
      (if (Variables|Default|GetShouldWaitAtEnd)
        (if (== (Variables|Default|GetAlpha) 1.0)
          (Utilities|FlowControl|Delay _timetostay)
          (CallFunction|Reverse)
          (elif (== (Variables|Default|GetAlpha) 0.0)
            (Utilities|FlowControl|Delay _timetostay)
            (CallFunction|Move)))))))

(event Custom|Reverse
  (bind _timetostay (Variables|Default|GetTimeToStay))
  (bind _trackref (Variables|Default|GetTrackRef))
  (bind _cameraspline (Variables|/Script/PROJ.CameraSpline|GetCameraSpline _trackref))
  (CallFunction|StartMovingSFX)
  (bind _alpha (Timeline|MoveToEnd Reverse)
    (:Update
      (Variables|Default|SetAlpha _alpha)
      (Transformation|SetActorLocationAndRotation (Spline|GetLocationatDistanceAlongSpline _cameraspline (Math|Float|Lerp 0.0 (Spline|GetSplineLength _cameraspline) (Variables|Default|GetAlpha)) "World") (Spline|GetRotationatDistanceAlongSpline (Variables|/Script/PROJ.CameraSpline|GetCameraSpline (Variables|Default|GetTrackRef)) (Math|Float|Lerp 0.0 (Spline|GetSplineLength _cameraspline) (Variables|Default|GetAlpha)) "Local")))
    (:Finished
      (CallFunction|LandedSFX)
      (if (Variables|Default|GetShouldWaitAtEnd)
        (if (== (Variables|Default|GetAlpha) 1.0)
          (Utilities|FlowControl|Delay _timetostay)
          (CallFunction|Reverse)
          (elif (== (Variables|Default|GetAlpha) 0.0)
            (Utilities|FlowControl|Delay _timetostay)
            (CallFunction|Move)))))))

(event EventTick
  (params (DeltaSeconds :type Float%20%28single-precision%29))
  (bind _currentgrid (Variables|Default|GetCurrentGrid))
  (Utilities|FlowControl|DoOnce false :!label _label
    (:Completed
      (Utilities|IsValid _currentgrid
        (:Is%20Valid
          (Class|Grid|CalculateMovingActor _currentgrid self)
          (Utilities|FlowControl|Delay 0.2)
          (goto _label Reset))))))

(event EventBeginPlay
  (bind _currentgrid (Variables|Default|GetCurrentGrid))
  (Utilities|FlowControl|Sequence
    (:then_0
      (if (Variables|Default|GetisLava)
        (Utilities|FlowControl|Delay (Variables|Default|GetWaitBeforeMove))
        (CallFunction|Move)))
    (:then_1
      (Utilities|IsValid _currentgrid
        (:Is%20Valid
          (Utilities|FlowControl|Delay 0.2)
          (Class|Grid|CalculateMovingActor _currentgrid self))))))

(fn ConstructionScript)