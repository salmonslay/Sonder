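; Player controller that applies saved player settings and tracks whether input comes from a gamepad.
; On BeginPlay it loads the save, copies its button mappings for local controllers, and sets game-only input.
; Saved brightness overwrites the InfiniteExtent post-process volume's settings as negated exposure limits, with a special offset for the Tutorial map.
; It also creates a second player when the game instance flags local play, and prints possessions for debugging.
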(event EventBeginPlay
  (Variables|Default|SetSaveFile (Class|PROJCharacter|GetSaveGameSafe))
  (CallFunction|SetBrightness)
  (CallFunction|LoadButtonMapping)
  (Variables|Default|SetbShowMouseCursor false)
  (Input|SetInputModeGameOnly self false)
  (bind _asbp_sonder_game_instance (Utilities|Casting|CastToBP_SonderGameInstance (Game|GetGameInstance)))
  (Variables|Default|SetAs%20BP%20Sonder%20Game%20Instance _asbp_sonder_game_instance)
  (Utilities|IsValid (Game|GetPlayerController 1)
    (:Is%20Not%20Valid
      (if (Variables|/Script/PROJ.SonderGameInstance|GetbIsPlayingLocal (Variables|Default|GetAs%20BP%20Sonder%20Game%20Instance))
        (Class|GameplayStatics|CreatePlayer -1)))))

(event EventPossess
  (params (PossessedPawn :type Pawn%20Object%20Reference))
  (Development|PrintString (Utilities|String|Append (Utilities|GetDisplayName PossessedPawn) " possessed by:  " (Utilities|GetDisplayName self)) true true "(R=1.000000,G=0.074582,B=0.000000,A=1.000000)" 5.0))

(event Input|KeyboardEvents|AnyKey
  (params (Key :type Key%20Structure))
  (bind _as_bp_sonder_game_instance (Variables|Default|GetAs%20BP%20Sonder%20Game%20Instance))
  (:Pressed
    (Utilities|IsValid _as_bp_sonder_game_instance
      (:Is%20Valid
        (Variables|/Game/Blueprints/BP_SonderGameInstance.BP_SonderGameInstance_C|SetUsingController _as_bp_sonder_game_instance (Class|KismetInputLibrary|KeyIsGamepadKey Key))))))

(fn ConstructionScript)

(fn LoadButtonMapping
  (bind _savefile (Variables|Default|GetSaveFile))
  (bind _inputmapping (LocalVariables|GetInputMapping))
  (bind _inputmappings (Variables|/Script/PROJ.SonderSaveGame|GetInputMappings _savefile))
  (bind _mappings (Variables|/Script/EnhancedInput.InputMappingContext|GetMappings _inputmapping))
  (if (Pawn|IsLocalPlayerController)
    (if (Utilities|Array|IsNotEmpty _inputmappings)
      (Utilities|Array|Clear _mappings)
      (for _array_element _inputmappings
        (Utilities|Array|Add _mappings _array_element)))))

(fn SetBrightness
  (bind _savefile (Variables|Default|GetSaveFile))
  (bind _brightness (Variables|/Script/PROJ.SonderSaveGame|GetBrightness _savefile))
  (bind _returnvalue (* _brightness -1.0))
  (bind _returnvalue_2 (+ -3.0 _returnvalue))
  (bind _outactors (Actor|GetAllActorsOfClasswithTag "/Script/Engine.PostProcessVolume" "InfiniteExtent"))
  (if (Utilities|Array|IsNotEmpty _outactors)
    (bind _returnvalue_3 (Game|GetCurrentLevelName true))
    (if (Utilities|Enum|NotEqual(Enum) _returnvalue_3 "Tutorial") ; Tutorial is a special case, only map that does not have brightness set to 0
      (Variables|/Script/Engine.PostProcessVolume|SetSettings (Utilities|Array|Get(acopy) _outactors) (Utilities|Struct|MakePostProcessSettings _returnvalue _returnvalue))
      (else
        (Variables|/Script/Engine.PostProcessVolume|SetSettings (Utilities|Array|Get(acopy) _outactors) (Utilities|Struct|MakePostProcessSettings _returnvalue_2 _returnvalue_2))))))