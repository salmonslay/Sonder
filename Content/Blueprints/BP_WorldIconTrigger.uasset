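; BP_WorldIconTrigger is a trigger actor that shows a world icon while qualifying actors are inside it.
; Overlap events track actors in a list, filtered by TriggeredBy: Robot requires the third-person character, Both accepts any actor, and otherwise only the soul character counts.
; Each tick, the icon's visibility follows whether that list is non-empty, and its image switches between controller and keyboard versions using the game instance's input flag.
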(event EventBeginPlay
  (Rendering|SetVisibility (Variables|/Game/Blueprints/BP_WorldIcon.BP_WorldIcon_C|GetWidget (Variables|Default|GetIconBlueprint)) false false)
  (bind _asbp_sonder_game_instance (Utilities|Casting|CastToBP_SonderGameInstance (Game|GetGameInstance)))
  (Variables|Default|SetAs%20BP%20Sonder%20Game%20Instance _asbp_sonder_game_instance))

(event Collision|EventActorBeginOverlap
  (params (OtherActor :type Actor%20Object%20Reference))
  (if (Utilities|Enum|NotEqual(Enum) (Variables|Default|GetTriggered%20by) "Both")
    (if (Utilities|Enum|Equal(Enum) (Variables|Default|GetTriggered%20by) "Robot")
      (Utilities|Casting|CastToBP_ThirdPersonCharacter OtherActor)
      (else
        (Utilities|Casting|CastToBP_SoulCharacter OtherActor))))
  (Utilities|Array|AddUnique (Variables|Default|GetActors%20in%20collider) OtherActor))

(event Collision|EventActorEndOverlap
  (params (OtherActor :type Actor%20Object%20Reference))
  (Utilities|Array|RemoveItem (Variables|Default|GetActors%20in%20collider) OtherActor))

(event EventTick
  (params (DeltaSeconds :type Float%20%28single-precision%29))
  (Utilities|FlowControl|Sequence
    (:then_0
      (Rendering|SetVisibility (Variables|/Game/Blueprints/BP_WorldIcon.BP_WorldIcon_C|GetWidget (Variables|Default|GetIconBlueprint)) (Utilities|Array|IsNotEmpty (Variables|Default|GetActors%20in%20collider)) false))
    (:then_1
      (Default|SetIcon (Variables|Default|GetIconBlueprint) (select (Variables|/Game/Blueprints/BP_SonderGameInstance.BP_SonderGameInstance_C|GetUsingController (Variables|Default|GetAs%20BP%20Sonder%20Game%20Instance)) (Variables|Default|GetController%20icon) (Variables|Default|GetKeyboard%20icon))))))

(fn ConstructionScript)

(fn EnableWidget)