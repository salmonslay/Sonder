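; BP_MoveBox is a movable box that drives FMOD sliding and landing sounds from its motion.
; Tick maps horizontal speed to the slideVelocity parameter, muting it during fast vertical motion, which also flags the box as airborne after a short delay.
; Hitting a static mesh while flagged clears the flag and plays BoxLand at the impact, with hitForce scaled by vertical speed times mass.
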(event Collision|EventHit
  (params (MyComp :type Primitive%20Component%20Object%20Reference) (Other :type Actor%20Object%20Reference) (OtherComp :type Primitive%20Component%20Object%20Reference) (bSelfMoved :type Boolean) (HitLocation :type Vector :default "0, 0, 0") (HitNormal :type Vector :default "0, 0, 0") (NormalImpulse :type Vector :default "0, 0, 0") (Hit :type Hit%20Result%20Structure%20%28by%20ref%29))
  (Utilities|Casting|CastToStaticMeshComponent OtherComp)
  (if (Variables|Default|GetinAirGuess)
    (Variables|Default|SetinAirGuess false)
    (bind _returnvalue (Class|FMODBlueprintStatics|PlayEventatLocation "/Game/FMOD/Events/SFX/BoxLand.BoxLand" (Math|Conversions|ToTransform(Vector) HitLocation)))
    (Class|FMODBlueprintStatics|EventInstanceSetParameter _returnvalue "hitForce" (Math|Float|Clamp(Float) (Math|Float|NormalizetoRange (* (Math|Vector|VectorLength (Math|Conversions|ToVector(Float) (.z (Transformation|GetVelocity)))) (Physics|GetMass (Variables|Debug|GetStaticMeshComponent))) 0.0 1.2e+05)))))

(event EventTick
  (params (DeltaSeconds :type Float%20%28single-precision%29))
  (bind _staticmeshcomponent (Variables|Debug|GetStaticMeshComponent))
  (bind _returnvalue (Transformation|GetComponentVelocity _staticmeshcomponent))
  (Class|FMODAudioComponent|SetParameter (Variables|Default|GetFMODAudio) "slideVelocity" (Math|Float|Absolute(Float) (Math|Float|Clamp(Float) (Math|Float|NormalizetoRange (+ (Math|Float|Absolute(Float) (.x _returnvalue)) (Math|Float|Absolute(Float) (.y _returnvalue))) 0.0 4e+02))))
  (if (> (Math|Float|Clamp(Float) (Math|Float|NormalizetoRange (Math|Float|Absolute(Float) (.z _returnvalue)) 0.0 1e+02)) 0.7)
    (Class|FMODAudioComponent|SetParameter (Variables|Default|GetFMODAudio) "slideVelocity" 0.0)
    (if (not (Variables|Default|GetairCountdownActivated))
      (Variables|Default|SetairCountdownActivated true)
      (Utilities|FlowControl|Delay 0.25)
      (Variables|Default|SetinAirGuess true)
      (Variables|Default|SetairCountdownActivated false))))

(fn ConstructionScript)