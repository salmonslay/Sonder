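; Spawner that brings a health pickup back into play at one of several preset spawn points when its trigger event fires, named for use in combat.
; TriggeredEvent unhides the referenced HealthPickUp, re-enables query-only collision on its sphere and teleports it to the current SpawnPoints entry.
; An index counter advances each trigger and wraps to zero, cycling the one reused pickup through the points in order.
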(event EventBeginPlay)

(event Collision|EventActorBeginOverlap
  (params (OtherActor :type Actor%20Object%20Reference)))

(event EventTick
  (params (DeltaSeconds :type Float%20%28single-precision%29)))

(event EventTriggeredEvent
  (bind _spawnpoints (Variables|Default|GetSpawnPoints))
  (bind _healthpickup (Variables|Default|GetHealthPickUp))
  (Utilities|IsValid _healthpickup
    (:Is%20Valid
      (Rendering|SetActorHiddenInGame _healthpickup false)
      (Collision|SetCollisionEnabled (Variables|/Game/Blueprints/Spawning/BP_HealthPickUp.BP_HealthPickUp_C|GetSphere _healthpickup) "QueryOnly")
      (Transformation|SetActorLocation _healthpickup (Transformation|GetActorLocation (Utilities|Array|Get(acopy) _spawnpoints (Variables|Default|GetIndexCounter))) false false)
      (bind _result (Math|Integer|IncrementInt (Variables|Default|GetIndexCounter))
        (:%20%20
          (if (>= _result (Utilities|Array|Length _spawnpoints))
            (Variables|Default|SetIndexCounter 0)))))))

(fn ConstructionScript)