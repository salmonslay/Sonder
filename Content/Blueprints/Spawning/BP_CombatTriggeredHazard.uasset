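; BP_CombatTriggeredHazard is a steam pipe hazard that damages overlapping PROJCharacters while active.
; TriggeredEvent activates the hazard and its Niagara steam effect, then switches both off after ActiveDuration.
; Begin and end overlap events maintain the OverlappingPlayers list.
; While active, Tick damages everyone in that list, using a DoOnce reset after a Delay to space hits by DamageTickFrequency.
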(event EventBeginPlay)

(event Collision|EventActorBeginOverlap
  (params (OtherActor :type Actor%20Object%20Reference))
  (bind _asprojcharacter (Utilities|Casting|CastToPROJCharacter OtherActor))
  (Utilities|Array|Add (Variables|Default|GetOverlappingPlayers) _asprojcharacter))

(event EventTick
  (params (DeltaSeconds :type Float%20%28single-precision%29))
  (if (Variables|Default|GetIsActive)
    (Utilities|FlowControl|DoOnce false :!label _label
      (:Completed
        (for _array_element (Variables|Default|GetOverlappingPlayers)
          (Class|PROJCharacter|TakeDamage _array_element (Variables|Default|GetDamage%20Amount) (Variables|Default|GetDamage%20Event) 0 self))
        (Utilities|FlowControl|Delay (Variables|Default|GetDamageTickFrequency))
        (goto _label Reset)))))

(event EventTriggeredEvent
  (Variables|Default|SetIsActive true)
  (Components|Activation|SetActive (Variables|Default|GetNS_SteamPipeStanding) true true)
  (Utilities|FlowControl|Delay (Variables|Default|GetActiveDuration))
  (Variables|Default|SetIsActive false)
  (Components|Activation|SetActive (Variables|Default|GetNS_SteamPipeStanding) false true))

(event Collision|EventActorEndOverlap
  (params (OtherActor :type Actor%20Object%20Reference))
  (bind _asprojcharacter (Utilities|Casting|CastToPROJCharacter OtherActor))
  (Utilities|Array|RemoveItem (Variables|Default|GetOverlappingPlayers) _asprojcharacter))

(fn ConstructionScript)