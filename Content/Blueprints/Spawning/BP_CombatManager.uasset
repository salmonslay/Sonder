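; Combat manager actor that drives music and kill-progress feedback for a combat encounter.
; On combat begin it starts FMOD music and, after a short delay, passes the enemy total to Progress; combat end plays a completion sound and stops the music.
; Each AddProgress call spawns a death wisp at the killed enemy, handing it Progress to advance the bar.
; Tick feeds the current wave into the music's Round parameter.
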(event Custom|AddProgress
  (params (KilledEnemy :type Enemy%20Character%20Object%20Reference))
  ;[1 1 1] Sends a particle from the enemy to the progress bar and fills it up one step
  (bind _returnvalue (Game|SpawnActorfromClass "/Game/Blueprints/BP_EnemyDeathWisp.BP_EnemyDeathWisp_C" (Math|Conversions|ToTransform(Vector) (Transformation|GetActorLocation KilledEnemy)) "Undefined" "MultiplyWithRoot" 0 0))
  (Default|EnemyDeath _returnvalue (Variables|Default|GetProgress)))

(event EventOnCombatBegin
  (bind _returnvalue (Class|FMODBlueprintStatics|PlayEvent2D (Variables|Default|GetMusic)))
  (Utilities|FlowControl|Delay 0.2)
  (Variables|/Game/Blueprints/BP_ArenaProgress.BP_ArenaProgress_C|SetTotalEnemies (Variables|Default|GetProgress) (Variables|Default|GetTotalEnemies)))

(event Collision|EventActorBeginOverlap
  (params (OtherActor :type Actor%20Object%20Reference)))

(event EventOnCombatEnd
  (Class|FMODBlueprintStatics|PlayEvent2D "/Game/FMOD/Events/SFX/CompletePuzzle.CompletePuzzle")
  (Class|FMODBlueprintStatics|EventInstanceStop (stale EventOnCombatBegin _returnvalue) true))

(event EventTick
  (params (DeltaSeconds :type Float%20%28single-precision%29))
  (Class|FMODBlueprintStatics|EventInstanceSetParameter (stale EventOnCombatBegin _returnvalue) "Round" (Math|Conversions|ToFloat(Integer) (Variables|Default|GetCurrentWave))))

(fn ConstructionScript)